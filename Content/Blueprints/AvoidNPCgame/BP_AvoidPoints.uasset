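; BP_AvoidPoints is a point pickup for the Avoid NPC game.
; When a BP_ThirdPersonCharacter overlaps its Box, it adds one to that character's AvoidNPCPoints and destroys itself.
; The first Tick starts Rotate through a DoOnce, and Rotate re-calls itself after a short Delay to step the Cube's yaw and alternate it up and down with a FlipFlop.
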(event `self.ReceiveTick`
  (params (DeltaSeconds :type "Float (single-precision)"))
  (`/Engine/EditorBlueprintResources/StandardMacros.DoOnce` false
    (:`Completed`
      (`self.Rotate`))))

(event `self.Box.OnComponentBeginOverlap`
  (params (OverlappedComponent :type "PrimitiveComponent Object Reference") (OtherActor :type "Actor Object Reference") (OtherComp :type "PrimitiveComponent Object Reference") (OtherBodyIndex :type Integer) (bFromSweep :type Boolean) (SweepResult :type "HitResult Structure (by ref)"))
  (bind _asbp_third_person_character (cast `/Game/ThirdPerson/Blueprints/BP_ThirdPersonCharacter` OtherActor))
  (set `/Game/ThirdPerson/Blueprints/BP_ThirdPersonCharacter.AvoidNPC Points` (+ (`/Game/ThirdPerson/Blueprints/BP_ThirdPersonCharacter.AvoidNPC Points` _asbp_third_person_character) 1.0) _asbp_third_person_character)
  (`self.K2_DestroyActor`))

(event `Rotate`
  (bind _cube (`self.Cube`))
  (bind _cube_2 (`self.Cube`))
  (bind _cube_3 (`self.Cube`))
  (bind (_returnvalue_x _returnvalue_y _returnvalue_z) (`KismetMathLibrary.BreakVector` (`SceneComponent.K2_GetComponentLocation` _cube_3)))
  (bind (_returnvalue_roll _returnvalue_pitch _returnvalue_yaw) (`KismetMathLibrary.BreakRotator` (`SceneComponent.K2_GetComponentRotation` _cube_2)))
  (bind (_returnvalue_x_2 _returnvalue_y_2 _returnvalue_z_2) (`KismetMathLibrary.BreakVector` (`SceneComponent.K2_GetComponentLocation` _cube)))
  (`|ExecutionSequence`
    (:`then_0`
      (`/Engine/EditorBlueprintResources/StandardMacros.FlipFlop`
        (:`A`
          (`SceneComponent.K2_SetWorldLocation` _cube_3 (`KismetMathLibrary.MakeVector` _returnvalue_x _returnvalue_y (+ _returnvalue_z 20.0)) false false))
        (:`B`
          (`SceneComponent.K2_SetWorldLocation` _cube (`KismetMathLibrary.MakeVector` _returnvalue_x_2 _returnvalue_y_2 (- _returnvalue_z_2 20.0)) false false))))
    (:`then_1`
      (`SceneComponent.K2_SetWorldRotation` _cube_2 (`KismetMathLibrary.MakeRotator` _returnvalue_roll _returnvalue_pitch (+ _returnvalue_yaw 50.0)) false false)
      (`KismetSystemLibrary.Delay` 0.2)
      (`self.Rotate`))))

(fn `UserConstructionScript`)