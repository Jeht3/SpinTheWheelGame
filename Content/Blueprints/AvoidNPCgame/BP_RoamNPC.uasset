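; BP_RoamNPC is a wandering NPC for the AvoidNPC game that slows the player on contact.
; From BeginPlay, MoveNPC sends it to a random reachable point within a radius of itself and immediately calls itself again on success or failure.
; An overlap on its Box component casts the other actor to BP_ThirdPersonCharacter and calls SlowDown on it.
; Two short Delay nodes leading into the retry calls are never triggered.
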(event `self.ReceiveBeginPlay`
  (`self.MoveNPC`))

(event `MoveNPC`
  (`|AIMoveTo` self (`NavigationSystemV1.K2_GetRandomReachablePointInRadius` (`self.K2_GetActorLocation`) 1000.0 null null) null
    (:`OnSuccess`
      (`self.MoveNPC`))
    (:`OnFail`
      (`self.MoveNPC`))))

(event `self.Box.OnComponentBeginOverlap`
  (params (OverlappedComponent :type "PrimitiveComponent Object Reference") (OtherActor :type "Actor Object Reference") (OtherComp :type "PrimitiveComponent Object Reference") (OtherBodyIndex :type Integer) (bFromSweep :type Boolean) (SweepResult :type "HitResult Structure (by ref)"))
  (bind _asbp_third_person_character (cast `/Game/ThirdPerson/Blueprints/BP_ThirdPersonCharacter` OtherActor))
  (`/Game/ThirdPerson/Blueprints/BP_ThirdPersonCharacter.SlowDown` _asbp_third_person_character))

(fn `UserConstructionScript`)