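; BP_AvoidNPCgame is the manager actor for a minigame built around avoiding roaming NPCs while gathering points.
; StartAvoidGame shows a timer widget and spawns BP_RoamNPC and BP_AvoidPoints actors at random reachable nav points around itself.
; Tick watches the player's AvoidNPCPoints until it reaches three.
; It then copies the timer value to TimeMultiplier, destroys the NPCs, completes the minigame on the player and removes the timer.
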(event `self.ReceiveTick`
  (params (DeltaSeconds :type "Float (single-precision)"))
  (bind _player_ref (`self.Player Ref`))
  (if (>= (`/Game/ThirdPerson/Blueprints/BP_ThirdPersonCharacter.AvoidNPC Points` (`self.Player Ref`)) 3.0)
    (`/Engine/EditorBlueprintResources/StandardMacros.DoOnce` false :!label _label
      (:`Completed`
        (set `/Game/ThirdPerson/Blueprints/BP_ThirdPersonCharacter.AvoidNPC Points` 0.0 _player_ref)
        (set `/Game/ThirdPerson/Blueprints/BP_ThirdPersonCharacter.TimeMultiplier` (`/Game/Blueprints/Widgets/WBP_Timer.Time` (`self.Timer Ref`)) _player_ref)
        (bind _outactors (`GameplayStatics.GetAllActorsOfClass` "/Game/Blueprints/AvoidNPCgame/BP_RoamNPC.BP_RoamNPC_C"))
        (for _array_element _outactors
          (`self.K2_DestroyActor` _array_element))
        (`/Game/ThirdPerson/Blueprints/BP_ThirdPersonCharacter.CompleteMinigame` (`self.Player Ref`))
        (`Widget.RemoveFromParent` (`self.Timer Ref`))
        (goto _label :!via `Reset`)))))

(event `self.ReceiveBeginPlay`
  (bind _returnvalue (`GameplayStatics.GetActorOfClass` "/Game/Blueprints/AvoidNPCgame/BP_RoamNPC.BP_RoamNPC_C"))
  (set `self.NPC ref` _returnvalue)
  (bind _asbp_third_person_character (cast `/Game/ThirdPerson/Blueprints/BP_ThirdPersonCharacter` (`GameplayStatics.GetPlayerCharacter` 0)))
  (set `self.Player Ref` _asbp_third_person_character))

(event `StartAvoidGame`
  (bind _returnvalue (`KismetMathLibrary.Conv_VectorToTransform` (`NavigationSystemV1.K2_GetRandomReachablePointInRadius` (`self.K2_GetActorLocation`) 10000.0 null null)))
  (bind _returnvalue_2 (`|CreateWidget` "/Game/Blueprints/Widgets/WBP_Timer.WBP_Timer_C" (`GameplayStatics.GetPlayerController` 0)))
  (set `self.Timer Ref` _returnvalue_2)
  (`UserWidget.AddToViewport` _returnvalue_2 0)
  (for _ (range 15)
    (`|SpawnActorFromClass` "/Game/Blueprints/AvoidNPCgame/BP_RoamNPC.BP_RoamNPC_C" _returnvalue "Undefined" "MultiplyWithRoot" null null))
  (for _ (range 3)
    (`|SpawnActorFromClass` "/Game/Blueprints/AvoidNPCgame/BP_AvoidPoints.BP_AvoidPoints_C" _returnvalue "Undefined" "MultiplyWithRoot" null null)))

(fn `UserConstructionScript`)