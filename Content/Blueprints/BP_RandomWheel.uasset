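; BP_RandomWheel is a wheel actor that spins when the third-person character overlaps its box, then launches a minigame.
; Each spin raises the player's game speed multiplier, with a timeline easing the arrow's yaw toward re-randomized targets.
; A line trace between two cubes then reads component colour tags.
; All four colours currently teleport the player to the chase game; the avoid, gather and falling branches are disconnected.
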(event `self.Box.OnComponentBeginOverlap`
  (params (OverlappedComponent :type "PrimitiveComponent Object Reference") (OtherActor :type "Actor Object Reference") (OtherComp :type "PrimitiveComponent Object Reference") (OtherBodyIndex :type Integer) (bFromSweep :type Boolean) (SweepResult :type "HitResult Structure (by ref)"))
  (bind _asbp_third_person_character (cast `/Game/ThirdPerson/Blueprints/BP_ThirdPersonCharacter` OtherActor))
  (set `self.Player Ref` _asbp_third_person_character)
  (`/Engine/EditorBlueprintResources/StandardMacros.DoOnce` false :!label _label
    (:`Completed`
      (`self.SpinWheel`)
      (`KismetSystemLibrary.Delay` 6.0)
      (goto _label :!via `Reset`))))

(event `SpinWheel`
  (bind _player_ref (`self.Player Ref`))
  (bind _arrow (`self.arrow`))
  (bind (_returnvalue_x _returnvalue_y _returnvalue_z) (`KismetMathLibrary.BreakVector` (`SceneComponent.K2_GetComponentLocation` (`self.Cube1`))))
  (bind (_relativerotation_roll _relativerotation_pitch) (`KismetMathLibrary.BreakRotator` (`SceneComponent.RelativeRotation` _arrow)))
  (bind (_relativerotation_roll_2 _relativerotation_pitch_2 _relativerotation_yaw) (`KismetMathLibrary.BreakRotator` (`SceneComponent.RelativeRotation` (`self.arrow`))))
  (set `/Game/ThirdPerson/Blueprints/BP_ThirdPersonCharacter.GameSpeedMultiplier` (* (`/Game/ThirdPerson/Blueprints/BP_ThirdPersonCharacter.GameSpeedMultiplier` _player_ref) 1.05) _player_ref)
  (bind (_direction _time) (`Timeline|RotateWheel` :!via `PlayFromStart`)
    (:`Update`
      (`SceneComponent.K2_SetRelativeRotation` _arrow (`KismetMathLibrary.MakeRotator` _relativerotation_roll _relativerotation_pitch (`KismetMathLibrary.FInterpTo` _relativerotation_yaw (`KismetMathLibrary.RandomFloatInRange` 360.0 2000.0) _time 0.01)) false false))
    (:`Finished`
      (`KismetSystemLibrary.Delay` 0.5)
      (bind _outhit (`KismetSystemLibrary.LineTraceSingle` :`Start` (`KismetMathLibrary.MakeVector` _returnvalue_x _returnvalue_y (+ _returnvalue_z 100.0)) :`End` (`SceneComponent.K2_GetComponentLocation` (`self.Cube2`)) :`TraceChannel` "TraceTypeQuery1" :`DrawDebugType` "ForDuration"))
      (for _array_element (`ActorComponent.ComponentTags` (`.HitComponent` (`GameplayStatics.BreakHitResult` _outhit)))
        (switch `string` (`KismetStringLibrary.Conv_NameToString` _array_element)
          (:`Blue`
            _)
          (:`Green`
            _)
          (:`Red`
            _)
          (:`Yellow`
            _))
        (`self.K2_SetActorLocation` (`GameplayStatics.GetPlayerCharacter` 0) (`self.K2_GetActorLocation` (`self.ChaseNPC Ref`)) false false)
        (`/Game/Blueprints/ChaseNPCgame/BP_ChaseNPCgame.StartChaseGame` (`self.ChaseNPC Ref`))))))

(fn `UserConstructionScript`)