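; BP_FallingPlate is a floor plate in the falling-avoidance minigame that becomes either a safe zone or a hazard.
; GuyFall and SafeZone events recolor it red or green, store the timer and re-arm the spawn.
; While the game runs, Tick watches the timer, spawning a BP_FallingGuy on unsafe plates below six seconds.
; Below three, a player inside the box receives a point on green or triggers GameOver on red.
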(event `self.ReceiveBeginPlay`
  (bind _asbp_third_person_character (cast `/Game/ThirdPerson/Blueprints/BP_ThirdPersonCharacter` (`GameplayStatics.GetPlayerCharacter` 0)))
  (set `self.Player Ref` _asbp_third_person_character))

(event `self.ReceiveTick`
  (params (DeltaSeconds :type "Float (single-precision)"))
  (bind _issafe_ (`self.IsSafe?`))
  (if (`/Game/ThirdPerson/Blueprints/BP_ThirdPersonCharacter.IsInFallingGame?` (`self.Player Ref`))
    (`|ExecutionSequence`
      (:`then_0`
        (if (< (`/Game/Blueprints/Widgets/WBP_Timer.Time` (`self.TimerRef`)) 6.0)
          (if (not _issafe_)
            (`/Engine/EditorBlueprintResources/StandardMacros.DoOnce` false :!label _label
              (:`Completed`
                (`|SpawnActorFromClass` "/Game/Blueprints/AvoidFallingGame/BP_FallingGuy.BP_FallingGuy_C" (`KismetMathLibrary.MakeTransform` (`SceneComponent.K2_GetComponentLocation` (`self.Cube1`))) "Undefined" "MultiplyWithRoot" null null))))))
      (:`then_1`
        (if (< (`/Game/Blueprints/Widgets/WBP_Timer.Time` (`self.TimerRef`)) 3.0)
          (if (`self.IsInCollider?`)
            (if _issafe_
              (`/Engine/EditorBlueprintResources/StandardMacros.DoOnce` false
                (:`Completed`
                  (set `/Game/ThirdPerson/Blueprints/BP_ThirdPersonCharacter.FallingPoints` 1.0 (`self.Player Ref`))))
              (else
                (`/Engine/EditorBlueprintResources/StandardMacros.DoOnce` false
                  (:`Completed`
                    (`/Game/ThirdPerson/Blueprints/BP_ThirdPersonCharacter.GameOver` (`self.Player Ref`))))))))))))

(event `GuyFall`
  (params (TimerRef :type "/Game/Blueprints/Widgets/WBP_Timer Object Reference"))
  (`self.Set Timer Ref` TimerRef)
  (`PrimitiveComponent.SetMaterial` (`self.Cube`) 0 "/AnimationSharing/AnimSharingRed.AnimSharingRed")
  (set `self.IsSafe?` false)
  (goto _label :!via `Reset`))

(event `SafeZone`
  (params (TimerRef :type "/Game/Blueprints/Widgets/WBP_Timer Object Reference"))
  (`self.Set Timer Ref` TimerRef)
  (`PrimitiveComponent.SetMaterial` (`self.Cube`) 0 "/AnimationSharing/AnimSharingGreen.AnimSharingGreen")
  (set `self.IsSafe?` true)
  (goto _label :!via `Reset`))

(event `Set Timer Ref`
  (params (TimerRef :type "/Game/Blueprints/Widgets/WBP_Timer Object Reference"))
  (set `self.TimerRef` TimerRef))

(event `self.Box.OnComponentBeginOverlap`
  (params (OverlappedComponent :type "PrimitiveComponent Object Reference") (OtherActor :type "Actor Object Reference") (OtherComp :type "PrimitiveComponent Object Reference") (OtherBodyIndex :type Integer) (bFromSweep :type Boolean) (SweepResult :type "HitResult Structure (by ref)"))
  (cast `/Game/ThirdPerson/Blueprints/BP_ThirdPersonCharacter` OtherActor)
  (set `self.IsInCollider?` true))

(event `self.Box.OnComponentEndOverlap`
  (params (OverlappedComponent :type "PrimitiveComponent Object Reference") (OtherActor :type "Actor Object Reference") (OtherComp :type "PrimitiveComponent Object Reference") (OtherBodyIndex :type Integer))
  (cast `/Game/ThirdPerson/Blueprints/BP_ThirdPersonCharacter` OtherActor)
  (set `self.IsInCollider?` false))

(fn `UserConstructionScript`)