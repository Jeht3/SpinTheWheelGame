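; Manager actor for a ball-gathering minigame in which the player must score five points while a timer widget is shown.
; StartGatherGame toggles the player's grabber, shows the timer and scatters BP_Balls at random reachable navmesh points around the actor.
; Tick polls the player's points, then copies the timer's time to TimeMultiplier, clears balls and timer, and completes the minigame.
; BeginPlay caches the player and an otherwise unused BP_FleeNPC reference.
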(event `self.ReceiveTick`
  (params (DeltaSeconds :type "Float (single-precision)"))
  (bind _player_ref (`self.Player Ref`))
  (if (>= (`/Game/ThirdPerson/Blueprints/BP_ThirdPersonCharacter.GatherBallsPoints` (`self.Player Ref`)) 5.0)
    (`/Engine/EditorBlueprintResources/StandardMacros.DoOnce` false :!label _label
      (:`Completed`
        (`/Game/ThirdPerson/Blueprints/BP_ThirdPersonCharacter.EnableDisableGrabber` _player_ref)
        (set `/Game/ThirdPerson/Blueprints/BP_ThirdPersonCharacter.GatherBallsPoints` 0.0 _player_ref)
        (set `/Game/ThirdPerson/Blueprints/BP_ThirdPersonCharacter.TimeMultiplier` (`/Game/Blueprints/Widgets/WBP_Timer.Time` (`self.Timer Ref`)) _player_ref)
        (bind _outactors (`GameplayStatics.GetAllActorsOfClass` "/Game/Blueprints/GatherBallsGame/BP_Balls.BP_Balls_C"))
        (for _array_element _outactors
          (`self.K2_DestroyActor` _array_element))
        (`/Game/ThirdPerson/Blueprints/BP_ThirdPersonCharacter.CompleteMinigame` (`self.Player Ref`))
        (`Widget.RemoveFromParent` (`self.Timer Ref`))
        (goto _label :!via `Reset`)))))

(event `self.ReceiveBeginPlay`
  (bind _returnvalue (`GameplayStatics.GetActorOfClass` "/Game/Blueprints/ChaseNPCgame/BP_FleeNPC.BP_FleeNPC_C"))
  (set `self.NPC ref` _returnvalue)
  (bind _asbp_third_person_character (cast `/Game/ThirdPerson/Blueprints/BP_ThirdPersonCharacter` (`GameplayStatics.GetPlayerCharacter` 0)))
  (set `self.Player Ref` _asbp_third_person_character))

(event `StartGatherGame`
  (`/Game/ThirdPerson/Blueprints/BP_ThirdPersonCharacter.EnableDisableGrabber` (`self.Player Ref`))
  (bind _returnvalue (`|CreateWidget` "/Game/Blueprints/Widgets/WBP_Timer.WBP_Timer_C" (`GameplayStatics.GetPlayerController` 0)))
  (set `self.Timer Ref` _returnvalue)
  (`UserWidget.AddToViewport` _returnvalue 0)
  (for _ (range 21)
    (`|SpawnActorFromClass` "/Game/Blueprints/GatherBallsGame/BP_Balls.BP_Balls_C" (`KismetMathLibrary.Conv_VectorToTransform` (`NavigationSystemV1.K2_GetRandomReachablePointInRadius` (`self.K2_GetActorLocation`) 10000.0 null null)) "Undefined" "MultiplyWithRoot" null null)))

(fn `UserConstructionScript`)