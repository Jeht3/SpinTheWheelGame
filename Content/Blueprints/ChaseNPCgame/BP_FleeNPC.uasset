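; An NPC for a chase game that flees from the player and can be caught by staying close to it.
; MoveNPC re-issues AI Move To every 0.2 seconds, picking a random reachable point around a spot directly away from the player.
; While the player overlaps its Box, a looping timer raises the player's CatchProgress and updates the catch bar widget.
; Tick turns that widget component toward the camera.
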(event `self.ReceiveBeginPlay`
  (`|ExecutionSequence`
    (:`then_0`
      (`self.PseudoTick`))
    (:`then_1`
      (bind _aswbp_catch_bar (cast `/Game/Blueprints/ChaseNPCgame/WBP_CatchBar` (`WidgetComponent.GetWidget` (`self.CatchBarWidget`))))
      (set `self.CatchBar Ref` _aswbp_catch_bar))
    (:`then_2`
      (bind _asbp_third_person_character (cast `/Game/ThirdPerson/Blueprints/BP_ThirdPersonCharacter` (`GameplayStatics.GetPlayerCharacter` 0)))
      (set `self.Player Ref` _asbp_third_person_character)
      (`self.MoveNPC`))))

(event `self.ReceiveTick`
  (params (DeltaSeconds :type "Float (single-precision)"))
  (bind _catchbarwidget (`self.CatchBarWidget`))
  (`SceneComponent.K2_SetWorldRotation` _catchbarwidget (`KismetMathLibrary.FindLookAtRotation` (`SceneComponent.K2_GetComponentLocation` _catchbarwidget) (`SceneComponent.K2_GetComponentLocation` (`PlayerCameraManager.TransformComponent` (`GameplayStatics.GetPlayerCameraManager` 0)))) false false))

(event `MoveNPC`
  (bind _returnvalue (`self.K2_GetActorLocation`))
  (`|AIMoveTo` self (`NavigationSystemV1.K2_GetRandomReachablePointInRadius` (`KismetMathLibrary.MakeVector` (.x (+ _returnvalue (* (`KismetMathLibrary.GetForwardVector` (`KismetMathLibrary.FindLookAtRotation` _returnvalue (`self.K2_GetActorLocation` (`self.Player Ref`)))) -500.0))) (.y (+ _returnvalue (* (`KismetMathLibrary.GetForwardVector` (`KismetMathLibrary.FindLookAtRotation` _returnvalue (`self.K2_GetActorLocation` (`self.Player Ref`)))) -500.0))) (.z _returnvalue)) 500.0 null null) null
    (:`then`
      (`KismetSystemLibrary.Delay` 0.2)
      (`self.MoveNPC`))))

(event `self.Box.OnComponentBeginOverlap`
  (params (OverlappedComponent :type "PrimitiveComponent Object Reference") (OtherActor :type "Actor Object Reference") (OtherComp :type "PrimitiveComponent Object Reference") (OtherBodyIndex :type Integer) (bFromSweep :type Boolean) (SweepResult :type "HitResult Structure (by ref)"))
  (cast `/Game/ThirdPerson/Blueprints/BP_ThirdPersonCharacter` OtherActor)
  (set `self.CanCatch?` true))

(event `self.Box.OnComponentEndOverlap`
  (params (OverlappedComponent :type "PrimitiveComponent Object Reference") (OtherActor :type "Actor Object Reference") (OtherComp :type "PrimitiveComponent Object Reference") (OtherBodyIndex :type Integer))
  (cast `/Game/ThirdPerson/Blueprints/BP_ThirdPersonCharacter` OtherActor)
  (set `self.CanCatch?` false))

(event `PseudoTick`
  (`KismetSystemLibrary.K2_SetTimerDelegate` (delegate `StartCatching?`) 0.1 true))

(event `StartCatching?`
  (bind _player_ref (`self.Player Ref`))
  (if (`self.CanCatch?`)
    (bind _output_get (set `/Game/ThirdPerson/Blueprints/BP_ThirdPersonCharacter.CatchProgress` (+ (`/Game/ThirdPerson/Blueprints/BP_ThirdPersonCharacter.CatchProgress` _player_ref) 3.0) _player_ref))
    (`ProgressBar.SetPercent` (`/Game/Blueprints/ChaseNPCgame/WBP_CatchBar.CatchBar` (`self.CatchBar Ref`)) (/ _output_get 100.0))))

(fn `UserConstructionScript`)